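; Player controller that lets the player switch control between the ThirdPersonCharacter instances placed in the level.
; On BeginPlay it gathers every ThirdPersonCharacter into an array and possesses the one at the current index.
; Pressing the SwitchCharacter input advances the index, wrapping to the first after the last, and possesses that character.
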(event EventBeginPlay
  (bind _outactors (Actor|GetAllActorsOfClass "/Game/ThirdPersonCPP/Blueprints/ThirdPersonCharacter.ThirdPersonCharacter_C"))
  (bind _output_get (Variables|Default|SetAvailableCharacters _outactors))
  (Pawn|Possess (Utilities|Array|Get(acopy) _output_get (Variables|Default|GetCurrentSelectedCharacterIndex))))

(event Input|ActionEvents|InputActionSwitchCharacter
  (params (Key :type Key%20Structure))
  (:Pressed
    (if (>= (Variables|Default|GetCurrentSelectedCharacterIndex) (- (Utilities|Array|Length (Variables|Default|GetAvailableCharacters)) 1))
      (Variables|Default|SetCurrentSelectedCharacterIndex 0)
      (else
        (Variables|Default|SetCurrentSelectedCharacterIndex (+ (Variables|Default|GetCurrentSelectedCharacterIndex) 1))))
    (Pawn|Possess (Utilities|Array|Get(acopy) (Variables|Default|GetAvailableCharacters) (Variables|Default|GetCurrentSelectedCharacterIndex)))))

(fn ConstructionScript)